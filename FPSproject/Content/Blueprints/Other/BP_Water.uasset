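; BP_Water is a rising water hazard that damages the player while they are inside it.
; A box overlap starts a printed timeline countdown that sets PlayerNear, letting Tick play the Wotah timeline to move the Niagara component on Z.
; Touching a BP_WLStop sets WaterLevel, which stops Tick replaying the timeline, and freezes that actor's physics collision.
; A second collision runs a looping timer that damages CBP_Health with red camera fades until overlap ends.
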(event `self.ReceiveTick`
  (params (DeltaSeconds :type "Float (single-precision)"))
  (set `self.Start` (`self.K2_GetActorLocation`))
  (if (`self.WaterLevel`)
    _
    (elif (`self.PlayerNear`)
      (bind (_direction _newtrack_0) (`Timeline|Wotah`)
        (:`Update`
          (`SceneComponent.K2_AddRelativeLocation` (`self.Niagara`) (`KismetMathLibrary.MakeVector` 0.0 0.0 _newtrack_0) false false))))))

(event `self.collision.OnComponentBeginOverlap`
  (params (OverlappedComponent :type "PrimitiveComponent Object Reference") (OtherActor :type "Actor Object Reference") (OtherComp :type "PrimitiveComponent Object Reference") (OtherBodyIndex :type Integer) (bFromSweep :type Boolean) (SweepResult :type "HitResult Structure (by ref)"))
  (bind _asbp_wlstop (cast `/Game/Blueprints/Other/BP_WLStop` OtherActor))
  (set `self.WaterLevel` true)
  (`PrimitiveComponent.SetSimulatePhysics` (`/Game/Blueprints/Other/BP_WLStop.BaxxaCollisi` _asbp_wlstop) false)
  (`PrimitiveComponent.SetPhysicsLinearVelocity` (`/Game/Blueprints/Other/BP_WLStop.BaxxaCollisi` _asbp_wlstop) (0.0 0.0 0.0) false "None"))

(event `self.Box.OnComponentBeginOverlap`
  (params (OverlappedComponent :type "PrimitiveComponent Object Reference") (OtherActor :type "Actor Object Reference") (OtherComp :type "PrimitiveComponent Object Reference") (OtherBodyIndex :type Integer) (bFromSweep :type Boolean) (SweepResult :type "HitResult Structure (by ref)"))
  (cast `/Game/InfimaGames/FreeFPSTemplate/Core/BP_Character` OtherActor)
  (bind (_direction _newtrack_0) (`Timeline|Timeline`)
    (:`Update`
      (bind _returnvalue (`KismetMathLibrary.Lerp` 0.0 30.0 _newtrack_0))
      (`KismetSystemLibrary.PrintString` (`KismetStringLibrary.Conv_DoubleToString` _returnvalue) true true (struct :`R` 0.875 :`G` 0.091146 :`B` 0.091146 :`A` 1.0) 30.0)
      (if (>= _returnvalue 30.0)
        (set `self.PlayerNear` true)
        (`KismetSystemLibrary.Delay` 10.0)))))

(event `self.collision1.OnComponentBeginOverlap`
  (params (OverlappedComponent :type "PrimitiveComponent Object Reference") (OtherActor :type "Actor Object Reference") (OtherComp :type "PrimitiveComponent Object Reference") (OtherBodyIndex :type Integer) (bFromSweep :type Boolean) (SweepResult :type "HitResult Structure (by ref)"))
  (bind _asbp_character (cast `/Game/InfimaGames/FreeFPSTemplate/Core/BP_Character` OtherActor))
  (bind _returnvalue (`KismetSystemLibrary.K2_SetTimerDelegate` (delegate `ApplyWaterDamage`) 2.0 true))
  (set `self.Timer Hndl` _returnvalue))

(event `ApplyWaterDamage`
  (bind _returnvalue (`GameplayStatics.GetPlayerController` 0))
  (bind _damageamt (`self.DamageAmt`))
  (`/Game/Core/Component/CBP_Health.Take Damage` (`self.GetComponentByClass` (stale `self.collision1.OnComponentBeginOverlap` _asbp_character) "/Game/Core/Component/CBP_Health.CBP_Health_C") _damageamt)
  (`KismetSystemLibrary.PrintString` (`KismetStringLibrary.Conv_DoubleToString` _damageamt))
  (`PlayerCameraManager.StartCameraFade` (`PlayerController.PlayerCameraManager` _returnvalue) 0.0 0.5 0.5 (struct :`R` 0.588542 :`A` 1.0) false false)
  (`KismetSystemLibrary.Delay` 0.2)
  (`PlayerCameraManager.StartCameraFade` (`PlayerController.PlayerCameraManager` _returnvalue) 0.5 0.0 1.0 (struct :`R` 0.182292 :`A` 1.0) false false))

(event `self.collision1.OnComponentEndOverlap`
  (params (OverlappedComponent :type "PrimitiveComponent Object Reference") (OtherActor :type "Actor Object Reference") (OtherComp :type "PrimitiveComponent Object Reference") (OtherBodyIndex :type Integer))
  (cast `/Game/InfimaGames/FreeFPSTemplate/Core/BP_Character` OtherActor)
  (`KismetSystemLibrary.K2_ClearAndInvalidateTimerHandle` (`self.Timer Hndl`)))

(fn `Fall`
  (`SceneComponent.K2_AddRelativeLocation` (`self.Niagara`) (0.0 0.0 -0.2) false false))

(fn `Rise`
  (`SceneComponent.K2_AddRelativeLocation` (`self.Niagara`) (0.0 0.0 0.0) false false))

(fn `UserConstructionScript`)