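; BP_Note is an interactable note that the player can open and close as an on-screen reading widget.
; Each IInteract call alternates through a FlipFlop, playing a page sound and either adding a WB_Note widget to the viewport or removing it.
; Look and move input are ignored while the note is open.
; A sphere overlap shows or hides a Widget component when something enters or leaves range.
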(event `/Game/Interface/IBP_Interaction.i_Interact`
  (params (Charecter :type "/Game/ThirdPerson/Blueprints/BP_ThirdPersonCharacter Object Reference"))
  (bind _returnvalue (`GameplayStatics.GetPlayerController` 0))
  (bind _returnvalue_2 (`SceneComponent.K2_GetComponentLocation` (`self.Note`)))
  (`/Engine/EditorBlueprintResources/StandardMacros.FlipFlop`
    (:`A`
      (`GameplayStatics.PlaySoundAtLocation` "/Game/Assets/Audio/Page_Cue.Page_Cue" _returnvalue_2 (struct) 1.0 1.0 0.0 null null null null)
      (bind _returnvalue_3 (`|CreateWidget` "/Game/Blueprints/Widget/Blueprints/WB_Note.WB_Note_C"))
      (`UserWidget.AddToViewport` _returnvalue_3 0)
      (`Controller.SetIgnoreLookInput` _returnvalue true)
      (`Controller.SetIgnoreMoveInput` _returnvalue true))
    (:`B`
      (`GameplayStatics.PlaySoundAtLocation` "/Game/Assets/Audio/Page_Cue.Page_Cue" _returnvalue_2 (struct) 1.0 1.0 0.0 null null null null)
      (`Widget.RemoveFromParent` _returnvalue_3)
      (`Controller.SetIgnoreLookInput` _returnvalue false)
      (`Controller.SetIgnoreMoveInput` _returnvalue false))))

(event `self.Sphere.OnComponentBeginOverlap`
  (params (OverlappedComponent :type "PrimitiveComponent Object Reference") (OtherActor :type "Actor Object Reference") (OtherComp :type "PrimitiveComponent Object Reference") (OtherBodyIndex :type Integer) (bFromSweep :type Boolean) (SweepResult :type "HitResult Structure (by ref)"))
  (`SceneComponent.SetVisibility` (`self.Widget`) true false))

(event `self.Sphere.OnComponentEndOverlap`
  (params (OverlappedComponent :type "PrimitiveComponent Object Reference") (OtherActor :type "Actor Object Reference") (OtherComp :type "PrimitiveComponent Object Reference") (OtherBodyIndex :type Integer))
  (`SceneComponent.SetVisibility` (`self.Widget`) false false))

(fn `UserConstructionScript`)