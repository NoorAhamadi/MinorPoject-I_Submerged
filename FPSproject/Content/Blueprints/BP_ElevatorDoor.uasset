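; BP_ElevatorDoor is a two-panel sliding elevator door that opens when a lever is pulled, then closes itself.
; On BeginPlay it binds ElevatorDoorOpen to the lever-pulled event on Cylinder.
; One timeline lerps D1 and D2 apart, with a five-second Delay chained from its Update pin leading into a second timeline that slides them back.
; CheckDoorOpen is an uncalled debug stub whose condition is always false.
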(event `self.ReceiveBeginPlay`
  (add `/Game/Blueprints/Puzzzle01/BP_Pull.LeverHasBeenPulled` (`self.Cylinder`) (delegate `Elevator Door Open`)))

(event `Elevator Door Open`
  (bind (_direction _newtrack_0) (`Timeline|ElevatorDoorOpen` :`NewTime` 2.0)
    (:`Update`
      (`SceneComponent.K2_SetRelativeLocation` (`self.D1`) (`KismetMathLibrary.VLerp` (-25.8 0.0 0.0) (-50.0 0.0 0.0) _newtrack_0) false false)
      (`SceneComponent.K2_SetRelativeLocation` (`self.D2`) (`KismetMathLibrary.VLerp` (0.0 0.0 0.0) (30.0 0.0 0.0) _newtrack_0) false false)
      (`KismetSystemLibrary.Delay` 5.0)
      (bind (_direction_2 _newtrack_0_2) (`Timeline|Timeline` :`NewTime` 2.0)
        (:`Update`
          (`SceneComponent.K2_SetRelativeLocation` (`self.D1`) (`KismetMathLibrary.VLerp` (-50.0 0.0 0.0) (-25.8 0.0 0.0) _newtrack_0_2) false false)
          (`SceneComponent.K2_SetRelativeLocation` (`self.D2`) (`KismetMathLibrary.VLerp` (30.0 0.0 0.0) (0.0 0.0 0.0) _newtrack_0_2) false false))))))

(fn `CheckDoorOpen`
  (`KismetSystemLibrary.PrintString` "Checking Door Open")
  (if (and false false)
    (`KismetSystemLibrary.PrintString` "Door is Opening")))

(fn `UserConstructionScript`)