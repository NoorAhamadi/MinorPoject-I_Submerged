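; BP_Light is a light Blueprint that makes its RectLight blink continuously during play.
; BeginPlay starts the LightBlink event, which steps the intensity from bright to dim to off with short delays between changes.
; The event calls itself at the end to loop indefinitely, using latent Delay nodes rather than a Timeline or timer.
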(event `self.ReceiveBeginPlay`
  (`self.Light Blink`))

(event `Light Blink`
  (`KismetSystemLibrary.Delay` 0.5)
  (`LightComponent.SetIntensity` (`self.RectLight`) 4000.0)
  (`KismetSystemLibrary.Delay` 0.6)
  (`LightComponent.SetIntensity` (`self.RectLight`) 1000.0)
  (`KismetSystemLibrary.Delay` 0.4)
  (`LightComponent.SetIntensity` (`self.RectLight`) 0.0)
  (`self.Light Blink`))

(fn `UserConstructionScript`)