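; BP_Pull is an interactable puzzle lever that toggles between two positions.
; While IsPulled is true, each interaction drives a FlipFlop that plays or reverses a Timeline rotating the Cylinder.
; Every Timeline update calls the LeverHasBeenPulled dispatcher and prints a debug message.
; A sphere overlap shows or hides the widget as BP_Character enters or leaves.
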(event `/Game/Interface/IBP_Interaction.i_Interact`
  (params (Charecter :type "/Game/ThirdPerson/Blueprints/BP_ThirdPersonCharacter Object Reference"))
  (if (`self.Is pulled`)
    (`/Engine/EditorBlueprintResources/StandardMacros.FlipFlop`
      (:`A`
        (bind (_direction _newtrack_0) (`Timeline|Timeline` :!label _label)
          (:`Update`
            (`SceneComponent.K2_SetRelativeRotation` (`self.Cylinder`) (`KismetMathLibrary.RLerp` (struct) (struct :`Roll` 60.0) _newtrack_0) false false)
            (`KismetSystemLibrary.PrintString` "Lever Pulled")
            (`self.LeverHasBeenPulled`))))
      (:`B`
        (goto _label :!via `Reverse`)))))

(event `self.Sph.OnComponentBeginOverlap`
  (params (OverlappedComponent :type "PrimitiveComponent Object Reference") (OtherActor :type "Actor Object Reference") (OtherComp :type "PrimitiveComponent Object Reference") (OtherBodyIndex :type Integer) (bFromSweep :type Boolean) (SweepResult :type "HitResult Structure (by ref)"))
  (cast `/Game/InfimaGames/FreeFPSTemplate/Core/BP_Character` OtherActor)
  (`SceneComponent.SetVisibility` (`self.Widget`) true false))

(event `self.Sph.OnComponentEndOverlap`
  (params (OverlappedComponent :type "PrimitiveComponent Object Reference") (OtherActor :type "Actor Object Reference") (OtherComp :type "PrimitiveComponent Object Reference") (OtherBodyIndex :type Integer))
  (cast `/Game/InfimaGames/FreeFPSTemplate/Core/BP_Character` OtherActor)
  (`SceneComponent.SetVisibility` (`self.Widget`) false false))

(fn `UserConstructionScript`)