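; Water actor whose Niagara effect moves vertically once the player has triggered it, until it meets a BP_WLStop.
; A character entering the Box starts a printed timeline count that, on completion, sets PlayerNear and destroys the Box.
; Tick then plays the Wotah timeline to offset the Niagara's height until Collision overlaps a stop, setting WaterLevel and freezing that stop's physics.
; Rise and Fall provide fixed-step nudges but are not called here.
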(event `self.ReceiveTick`
  (params (DeltaSeconds :type "Float (single-precision)"))
  (if (`self.WaterLevel`)
    _
    (elif (`self.PlayerNear`)
      (bind (_direction _newtrack_0) (`Timeline|Wotah`)
        (:`Update`
          (`SceneComponent.K2_AddRelativeLocation` (`self.Niagara`) (`KismetMathLibrary.MakeVector` 0.0 0.0 _newtrack_0) false false))))))

(event `self.collision.OnComponentBeginOverlap`
  (params (OverlappedComponent :type "PrimitiveComponent Object Reference") (OtherActor :type "Actor Object Reference") (OtherComp :type "PrimitiveComponent Object Reference") (OtherBodyIndex :type Integer) (bFromSweep :type Boolean) (SweepResult :type "HitResult Structure (by ref)"))
  (bind _asbp_wlstop (cast `/Game/Blueprints/BP_WLStop` OtherActor))
  (set `self.WaterLevel` true)
  (`PrimitiveComponent.SetSimulatePhysics` (`/Game/Blueprints/BP_WLStop.BaxxaCollisi` _asbp_wlstop) false)
  (`PrimitiveComponent.SetPhysicsLinearVelocity` (`/Game/Blueprints/BP_WLStop.BaxxaCollisi` _asbp_wlstop) (0.0 0.0 0.0) false "None"))

(event `self.Box.OnComponentBeginOverlap`
  (params (OverlappedComponent :type "PrimitiveComponent Object Reference") (OtherActor :type "Actor Object Reference") (OtherComp :type "PrimitiveComponent Object Reference") (OtherBodyIndex :type Integer) (bFromSweep :type Boolean) (SweepResult :type "HitResult Structure (by ref)"))
  (cast `/Game/InfimaGames/FreeFPSTemplate/Core/BP_Character` OtherActor)
  (bind (_direction _newtrack_0) (`Timeline|Timeline`)
    (:`Update`
      (bind _returnvalue (`KismetMathLibrary.Lerp` 0.0 30.0 _newtrack_0))
      (`KismetSystemLibrary.PrintString` (`KismetStringLibrary.Conv_DoubleToString` _returnvalue) true true (struct :`R` 0.875 :`G` 0.091146 :`B` 0.091146 :`A` 1.0) 30.0)
      (if (>= _returnvalue 30.0)
        (set `self.PlayerNear` true)
        (`ActorComponent.K2_DestroyComponent` (`self.Box`))
        (`KismetSystemLibrary.Delay` 10.0)))))

(fn `Fall`
  (`SceneComponent.K2_AddRelativeLocation` (`self.Niagara`) (0.0 0.0 -0.5) false false))

(fn `Rise`
  (`SceneComponent.K2_AddRelativeLocation` (`self.Niagara`) (0.0 0.0 0.5) false false))

(fn `UserConstructionScript`)