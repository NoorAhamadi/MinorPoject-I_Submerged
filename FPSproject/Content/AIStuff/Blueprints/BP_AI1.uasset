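; BP_AI1 is an AI pawn that walks toward a fixed point when play begins.
; BeginPlay starts a walking montage, sets a slow walk speed and issues AIMoveTo to a hard-coded destination.
; Its PawnSensing see-pawn event is empty, and a chase that plays an attack montage on arrival is disconnected, as is an unused random reachable point lookup.
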(event `self.ReceiveBeginPlay`
  (`|PlayMontage` (`self.Mesh`) "/Game/AI/Animations/Walking__Montage.Walking__Montage"
    (:`then`
      (set `CharacterMovementComponent.MaxWalkSpeed` 150.0 (`self.CharacterMovement`))
      (`|AIMoveTo` self (1000.0 0.0 0.0) null))))

(event `self.PawnSensing.OnSeePawn`
  (params (Pawn :type "Pawn Object Reference")))

(fn `UserConstructionScript`)