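; Enemy AI character that roams random reachable points, chases pawns seen by PawnSensing and melee-attacks them.
; A retriggerable delay resumes roaming after sightings stop; reaching the target plays an attack montage whose notify sphere-traces between two arrows to damage CBP_Health components.
; Any damage reduces its own Health, ragdolls it at zero or below, and destroys it five seconds later regardless.
; A sphere overlap with BP_Character plays a monster sound.
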(event `self.ReceiveAnyDamage`
  (params (Damage :type "Float (single-precision)") (DamageType :type "DamageType Object Reference") (InstigatedBy :type "Controller Object Reference") (DamageCauser :type "Actor Object Reference"))
  ;[1 0.08915 0 1 11] This is where we ragdoll the entire character, it is as simple as this, yep!
  (bind _output_get (set `self.Health` (- (`self.Health`) Damage)))
  (`KismetSystemLibrary.PrintString` (`KismetStringLibrary.Conv_DoubleToString` _output_get))
  (`PrimitiveComponent.SetSimulatePhysics` (`self.Mesh`) (<= _output_get 0.0))
  (`KismetSystemLibrary.Delay` 5.0)
  (`self.K2_DestroyActor`))

(event `self.Sphere.OnComponentBeginOverlap`
  (params (OverlappedComponent :type "PrimitiveComponent Object Reference") (OtherActor :type "Actor Object Reference") (OtherComp :type "PrimitiveComponent Object Reference") (OtherBodyIndex :type Integer) (bFromSweep :type Boolean) (SweepResult :type "HitResult Structure (by ref)"))
  (cast `/Game/InfimaGames/FreeFPSTemplate/Core/BP_Character` OtherActor)
  (`GameplayStatics.PlaySoundAtLocation` "/Game/Sounds/monster-fx-sound-1-94403.monster-fx-sound-1-94403" (`SceneComponent.K2_GetComponentLocation` (`self.Mesh`)) (struct) 1.0 1.0 0.0 null null null null))

(event `self.CBP_Health.ED_DamageTaken`)

(event `self.CBP_Health.ED_Death`)

(event `self.ReceiveBeginPlay`
  (`self.Roaming`))

(event `Roaming`
  (set `CharacterMovementComponent.MaxWalkSpeed` 150.0 (`self.CharacterMovement`))
  (`|AIMoveTo` self (`NavigationSystemV1.K2_GetRandomReachablePointInRadius` (`SceneComponent.K2_GetComponentLocation` (`self.Mesh`)) 800.0 null null) null
    (:`then`
      _)
    (:`OnSuccess`
      _))
  (`KismetSystemLibrary.Delay` (`KismetMathLibrary.RandomFloatInRange` 1.0 4.0))
  (`self.Roaming`))

(event `self.PawnSensing.OnSeePawn`
  (params (Pawn :type "Pawn Object Reference"))
  (set `CharacterMovementComponent.MaxWalkSpeed` 100.0 (`self.CharacterMovement`))
  (`|ExecutionSequence`
    (:`then_0`
      (`|AIMoveTo` self (0.0 0.0 0.0) Pawn 2.0
        (:`OnSuccess`
          (`self.Attack`))))
    (:`then_1`
      (`KismetSystemLibrary.RetriggerableDelay` 2.0)
      (`self.Roaming`))))

(event `Walking`
  (`|PlayMontage` (`self.Mesh`) "/Game/AI/Animations/Walking__Montage.Walking__Montage"
    (:`then`
      (set `CharacterMovementComponent.MaxWalkSpeed` 150.0 (`self.CharacterMovement`))
      (`|AIMoveTo` self (0.0 0.0 0.0) null))))

(event `Attack`
  (`/Engine/EditorBlueprintResources/StandardMacros.DoOnce` false :!label _label
    (:`Completed`
      (set `self.is Attacking` true)
      (`CharacterMovementComponent.DisableMovement` (`self.CharacterMovement`))
      (`|PlayMontage` (`self.Mesh`) "/Game/AI/Animations/AI_Attack.AI_Attack"
        (:`OnCompleted`
          (`KismetSystemLibrary.PrintString` "Is attacking")
          (`CharacterMovementComponent.SetMovementMode` (`self.CharacterMovement`) "MOVE_Walking" 0 :!label _label_2)
          (goto _label :!via `Reset`))
        (:`OnInterrupted`
          (`KismetSystemLibrary.Delay` 1.0)
          (goto _label_2))
        (:`OnNotifyBegin`
          (`self.Deal Damage`))))))

(event `Deal Damage`
  (bind (_outhit _returnvalue) (`KismetSystemLibrary.SphereTraceSingle` :`Start` (`SceneComponent.K2_GetComponentLocation` (`self.Arrow1`)) :`End` (`SceneComponent.K2_GetComponentLocation` (`self.Arrow2`)) :`Radius` 30.0 :`TraceChannel` "TraceTypeQuery1" :`DrawDebugType` "ForDuration"))
  (for _array_element (`|MakeArray` _outhit)
    (if _returnvalue
      (bind _returnvalue_2 (`self.GetComponentByClass` (`.HitActor` (`GameplayStatics.BreakHitResult` _array_element)) "/Game/Core/Component/CBP_Health.CBP_Health_C"))
      (`/Engine/EditorBlueprintResources/StandardMacros.IsValid` _returnvalue_2
        (:`Is Valid`
          (`/Game/Core/Component/CBP_Health.Take Damage` _returnvalue_2 (`self.Damage Amount`))
          (`KismetSystemLibrary.PrintString` "Character is losing HP")))
      (else
        (`KismetSystemLibrary.PrintString` "No Damage Done")))))

(event `self.ReceiveTick`
  (params (DeltaSeconds :type "Float (single-precision)"))
  (if (> (`KismetMathLibrary.VSize` (`self.GetVelocity` self)) 0.0)
    (if (not (`self.is Attacking`))
      (`|PlayMontage` (`self.Mesh`) "/Game/AI/Animations/AI_Attack.AI_Attack"))))

(fn `UserConstructionScript`)