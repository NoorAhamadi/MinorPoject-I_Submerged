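; BP_AI_Jombiee is an enemy AI actor with health, a proximity sound and an attack animation.
; Damage lowers and prints health, ragdolls the mesh at zero or below, and destroys the actor five seconds later, even if health remains.
; One sphere overlap plays a monster sound for BP_Character; the other prints any overlapping actor and plays the attack montage, without applying damage.
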(event `self.ReceiveAnyDamage`
  (params (Damage :type "Float (single-precision)") (DamageType :type "DamageType Object Reference") (InstigatedBy :type "Controller Object Reference") (DamageCauser :type "Actor Object Reference"))
  ;[1 0.08915 0 1 11] This is where we ragdoll the entire character, it is as simple as this, yep!
  (bind _output_get (set `self.Health` (- (`self.Health`) Damage)))
  (`KismetSystemLibrary.PrintString` (`KismetStringLibrary.Conv_DoubleToString` _output_get))
  (`PrimitiveComponent.SetSimulatePhysics` (`self.SkeletalMesh`) (<= _output_get 0.0))
  (`KismetSystemLibrary.Delay` 5.0)
  (`self.K2_DestroyActor`))

(event `self.Sphere.OnComponentBeginOverlap`
  (params (OverlappedComponent :type "PrimitiveComponent Object Reference") (OtherActor :type "Actor Object Reference") (OtherComp :type "PrimitiveComponent Object Reference") (OtherBodyIndex :type Integer) (bFromSweep :type Boolean) (SweepResult :type "HitResult Structure (by ref)"))
  (cast `/Game/InfimaGames/FreeFPSTemplate/Core/BP_Character` OtherActor)
  (`GameplayStatics.PlaySoundAtLocation` "/Game/Sounds/monster-fx-sound-1-94403.monster-fx-sound-1-94403" (`SceneComponent.K2_GetComponentLocation` (`self.SkeletalMesh`)) (struct) 1.0 1.0 0.0 null null null null))

(event `self.Sphere1.OnComponentBeginOverlap`
  (params (OverlappedComponent :type "PrimitiveComponent Object Reference") (OtherActor :type "Actor Object Reference") (OtherComp :type "PrimitiveComponent Object Reference") (OtherBodyIndex :type Integer) (bFromSweep :type Boolean) (SweepResult :type "HitResult Structure (by ref)"))
  (`KismetSystemLibrary.PrintString` (`KismetSystemLibrary.GetDisplayName` OtherActor))
  (`|PlayMontage` (`self.SkeletalMesh`) "/Game/AI/Animations/AI_Attack.AI_Attack" 1.0 0.0 "None" false))

(fn `UserConstructionScript`)